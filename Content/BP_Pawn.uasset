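; BP_Pawn is a pawn with a zoomable spring-arm camera.
; On BeginPlay it casts its controller to PC_LevelController and adds the IMC_Level Enhanced Input mapping context.
; The CameraZoom action changes the arm length by a scaled input value while the current length lies within the Closeview and FarView limits.
; The new length is not clamped, so a step can overshoot those limits.
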(event Input|EnhancedActionEvents|EnhancedInputActionCameraZoom
  (params (ActionValue :type Float%20%28double-precision%29) (ElapsedSeconds :type Float%20%28double-precision%29) (TriggeredSeconds :type Float%20%28double-precision%29) (InputAction :type Input%20Action%20Object%20Reference :default "/Game/Inputs/CameraZoom.CameraZoom"))
  (bind _springarm (Variables|Default|GetSpringArm))
  ;[0 0 0] Camera Zoom In/Out
  (if (and (< (- (Variables|/Script/Engine.SpringArmComponent|GetTargetArmLength (Variables|Default|GetSpringArm)) 1.0) (Variables|Default|GetFarView)) (> (+ (Variables|/Script/Engine.SpringArmComponent|GetTargetArmLength (Variables|Default|GetSpringArm)) 1.0) (Variables|Default|GetCloseview)))
    (Variables|/Script/Engine.SpringArmComponent|SetTargetArmLength _springarm (+ (* ActionValue 99.0) (Variables|/Script/Engine.SpringArmComponent|GetTargetArmLength _springarm)))))

(event EventBeginPlay
  (bind _aspc_level_controller (Utilities|Casting|CastToPC_LevelController (Pawn|GetController)))
  (Input|AddMappingContext (PlayerController|LocalPlayerSubsystems|GetEnhancedInputLocalPlayerSubsystem _aspc_level_controller) "/Game/Inputs/IMC_Level.IMC_Level" 0 "(bIgnoreAllPressedKeysUntilRelease=True,bForceImmediately=False,bNotifyUserSettings=False)"))

(fn ConstructionScript)