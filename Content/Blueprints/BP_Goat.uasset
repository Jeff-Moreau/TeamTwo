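; BP_Goat is a goat actor that travels along a BP_GoatSpline path once the global start button flag is set.
; BeginPlay caches GI_Globals, sets Speed and keeps the last BP_GoatSpline found in the level.
; While GStartButton is true, Tick calls FollowSpline, which plays a timeline at a rate of 1/Speed.
; Timeline updates lerp distance along the spline, setting location in world space and rotation in local space.
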(event Custom|FollowSpline
  (Components|Timeline|SetPlayRate (Variables|Default|GetGoat_Time) (/ 1.0 (Variables|Default|GetSpeed)))
  (bind _newtrack_0 (Timeline|Goat_Time Play)
    (:Update
      (Variables|Default|SetSplineDistance (Math|Float|Lerp 0.0 (Spline|GetSplineLength (Variables|/Game/Blueprints/BP_GoatSpline.BP_GoatSpline_C|GetSpline (Variables|Default|GetGoatSpline))) _newtrack_0))
      (Transformation|SetActorTransform (Math|Transform|MakeTransform (Spline|GetLocationatDistanceAlongSpline (Variables|/Game/Blueprints/BP_GoatSpline.BP_GoatSpline_C|GetSpline (Variables|Default|GetGoatSpline)) (Variables|Default|GetSplineDistance) "World") (Spline|GetRotationatDistanceAlongSpline (Variables|/Game/Blueprints/BP_GoatSpline.BP_GoatSpline_C|GetSpline (Variables|Default|GetGoatSpline)) (Variables|Default|GetSplineDistance) "Local") "1.000000,1.000000,1.000000")))))

(event EventBeginPlay
  (bind _asgi_globals (Utilities|Casting|CastToGI_Globals (Game|GetGameInstance)))
  (Variables|Default|SetGlobals _asgi_globals)
  (Variables|Default|SetSpeed 15.0)
  (bind _outactors (Actor|GetAllActorsOfClass "/Game/Blueprints/BP_GoatSpline.BP_GoatSpline_C"))
  (for _array_element _outactors
    (Variables|Default|SetGoatSpline _array_element)))

(event Collision|EventActorBeginOverlap
  (params (OtherActor :type Actor%20Object%20Reference)))

(event EventTick
  (params (DeltaSeconds :type Float%20%28single-precision%29))
  (if (Variables|/Game/GI_Globals.GI_Globals_C|GetGStartButton (Variables|Default|GetGlobals))
    (CallFunction|FollowSpline)))

(fn ConstructionScript)