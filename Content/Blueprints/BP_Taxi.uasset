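; BP_Taxi is a vehicle actor that drives along the nearest BP_TestSpline once the global start button is pressed.
; Setup picks a random Niagara color and derives speed from GI_Globals; Tick then plays a timeline that moves the taxi by spline distance.
; Overlapping another car, taxi, truck or bus spawns an explosion and destroys it.
; Finishing intact decrements the global arrived-car counter and spawns fireworks.
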(event Custom|FollowSpline
  (Components|Timeline|SetPlayRate (Variables|Default|GetT_FollowSpline) (/ 1.0 (Variables|Default|GetSpeed)))
  (bind _testspline (Timeline|T_FollowSpline Play)
    (:Update
      (Variables|Default|SetSplineDistance (Math|Float|Lerp 0.0 (Spline|GetSplineLength (Variables|/Game/Blueprints/BP_TestSpline.BP_TestSpline_C|GetSpline (Variables|Default|GetTestSpline))) _testspline))
      (Transformation|SetActorTransform (Math|Transform|MakeTransform (Spline|GetLocationatDistanceAlongSpline (Variables|/Game/Blueprints/BP_TestSpline.BP_TestSpline_C|GetSpline (Variables|Default|GetTestSpline)) (Variables|Default|GetSplineDistance) "World") (Spline|GetRotationatDistanceAlongSpline (Variables|/Game/Blueprints/BP_TestSpline.BP_TestSpline_C|GetSpline (Variables|Default|GetTestSpline)) (Variables|Default|GetSplineDistance) "Local") "1.000000,1.000000,1.000000")))
    (:Finished
      (Utilities|FlowControl|DoN 1
        (:Exit
          (if (not (Variables|Default|GetDeadCar))
            (Variables|/Game/GI_Globals.GI_Globals_C|SetGTotalCarsArrived (Variables|Default|GetGlobals) (+ (Variables|/Game/GI_Globals.GI_Globals_C|GetGTotalCarsArrived (Variables|Default|GetGlobals)) -1))
            (Utilities|FlowControl|DoN 1
              (:Exit
                (Variables|Default|SetCanBeGoated false)
                (Game|SpawnActorfromClass "/Game/Blueprints/BP_Fireworks.BP_Fireworks_C" (Math|Transform|MakeTransform (.location (Transformation|GetActorTransform)) "0, 0, 0" "1.000000,1.000000,1.000000") "Undefined" "MultiplyWithRoot" 0 0)))))))))

(event EventBeginPlay
  (CallFunction|InitializeGlobals)
  (CallFunction|InitializeVariables)
  (Niagara|SetNiagaraVariable(LinearColor) (Variables|Default|GetNiagara) "User.SetColor" (.OutItem (Utilities|Array|Random (Variables|Default|Getniagracolor)))))

(event Collision|EventActorBeginOverlap
  (params (OtherActor :type Actor%20Object%20Reference))
  (bind _returnvalue (Utilities|GetClass OtherActor))
  (if (Math|Boolean|ORBoolean (== _returnvalue "/Game/Blueprints/BP_Car.BP_Car_C") (== _returnvalue "BP_Taxi_C") (== _returnvalue "/Game/Blueprints/BP_Truck.BP_Truck_C") (== _returnvalue "/Game/Blueprints/BP_Bus.BP_Bus_C"))
    (Variables|Default|SetDeadCar true)
    (Game|SpawnActorfromClass "/Game/Blueprints/BP_Explosion.BP_Explosion_C" (Math|Transform|MakeTransform (.location (Transformation|GetActorTransform)) "0, 0, 0" "1.000000,1.000000,1.000000") "Undefined" "MultiplyWithRoot" 0 0)
    (Audio|Components|Audio|Stop (Variables|Default|GetT_FollowSpline))
    (Actor|DestroyActor)))

(event EventTick
  (params (DeltaSeconds :type Float%20%28single-precision%29))
  (if (Variables|/Game/GI_Globals.GI_Globals_C|GetGStartButtonPressed (Variables|Default|GetGlobals))
    (CallFunction|FollowSpline)))

(fn ConstructionScript)

(fn InitializeGlobals
  (bind _asgi_globals (Utilities|Casting|CastToGI_Globals (Game|GetGameInstance)))
  (Variables|Default|SetGlobals _asgi_globals))

(fn InitializeVariables
  (Variables|Default|SetSpeedMultiplier 1.0)
  (Variables|Default|SetSpeed (* (Variables|/Game/GI_Globals.GI_Globals_C|GetGVehicleBaseSpeed (Variables|Default|GetGlobals)) (Variables|Default|GetSpeedMultiplier)))
  (Variables|Default|SetClosestSpline 1e+04)
  (bind _testspline (CallFunction|NearestSpline))
  (Variables|Default|SetTestSpline _testspline)
  (Variables|Default|SetDidSpawnTrace true)
  (Variables|Default|SetDeadCar false)
  (Variables|Default|SetCanBeGoated true))

(fn NearestSpline
  (bind _outactors (Actor|GetAllActorsOfClass "/Game/Blueprints/BP_TestSpline.BP_TestSpline_C"))
  (for _array_element _outactors
    (if (and (< (Transformation|GetDistanceTo _array_element) (Variables|Default|GetClosestSpline)) (> (Transformation|GetDistanceTo _array_element) 0.0))
      (Variables|Default|SetTestSpline _array_element)
      (Variables|Default|SetClosestSpline (Transformation|GetDistanceTo _array_element))))
  (return (Variables|Default|GetTestSpline)))

(fn SpawnTrace)